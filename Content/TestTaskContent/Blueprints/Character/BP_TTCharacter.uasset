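; BP_TTCharacter is a character Blueprint that lets the character toggle the message visibility of interactable actors it overlaps.
; Capsule overlap events store any actor implementing BPI_Settingable as CurrentInteract, and clear it when such an actor leaves the overlap.
; The TryToInteract event checks that this reference is valid, reads its message visibility and sets it to the opposite state.
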(event OnComponentBeginOverlap(CapsuleComponent)
  (params (OverlappedComponent :type Primitive%20Component%20Object%20Reference) (OtherActor :type Actor%20Object%20Reference) (OtherComp :type Primitive%20Component%20Object%20Reference) (OtherBodyIndex :type Integer) (bFromSweep :type Boolean) (SweepResult :type Hit%20Result%20Structure%20%28by%20ref%29))
  (if (Utilities|DoesObjectImplementInterface OtherActor "/Game/TestTaskContent/Blueprints/Interfaces/BPI_Settingable.BPI_Settingable_C")
    (Variables|Default|SetCurrentInteract OtherActor)))

(event OnComponentEndOverlap(CapsuleComponent)
  (params (OverlappedComponent :type Primitive%20Component%20Object%20Reference) (OtherActor :type Actor%20Object%20Reference) (OtherComp :type Primitive%20Component%20Object%20Reference) (OtherBodyIndex :type Integer))
  (if (Utilities|DoesObjectImplementInterface OtherActor "/Game/TestTaskContent/Blueprints/Interfaces/BPI_Settingable.BPI_Settingable_C")
    (Variables|Default|SetCurrentInteract 0)))

(event Custom|TryToInteract
  (bind _currentinteract (Variables|Default|GetCurrentInteract)
    (:then
      (bind _bisvisible (Class|BPISettingable|GetVisibility(Message) _currentinteract))
      (if _bisvisible
        (Class|BPISettingable|ChangeVisibility(Message) _currentinteract false)
        (else
          (Class|BPISettingable|ChangeVisibility(Message) _currentinteract true))))
    (:else)))

(fn ConstructionScript)