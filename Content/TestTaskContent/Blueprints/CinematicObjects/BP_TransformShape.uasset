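; BP_TransformShape is a cinematic object that changes its static mesh shape and then slides along the X axis.
; On BeginPlay it applies the default mesh, waits briefly, spawns a water-ball hit particle burst, and swaps in the transform mesh.
; The Move event then plays the MeshMovement timeline, remapping its XOffset to lerp world X from the starting position to TargetXLocation, keeping Y and Z.
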(event Custom|Move
  (bind _staticmesh (Variables|Default|GetStaticMesh))
  (bind _returnvalue (Transformation|GetWorldLocation _staticmesh))
  (bind _xoffset (Timeline|MeshMovement PlayFromStart)
    (:Update
      (Transformation|SetWorldLocation _staticmesh (Math|Vector|MakeVector (Math|Float|MapRangeClamped _xoffset 0.0 1.0 (Variables|Default|GetCurrentXLocation) (Variables|Default|GetTargetXLocation)) (.y _returnvalue) (.z _returnvalue)) false false))))

(event EventBeginPlay
  (bind _staticmesh (Variables|Default|GetStaticMesh)
    (:then
      (Variables|Default|SetCurrentXLocation (.x (Transformation|GetWorldLocation _staticmesh)))
      (Components|StaticMesh|SetStaticMesh _staticmesh (Variables|Settings|GetDefaultMesh))
      (Utilities|FlowControl|Delay 1.0)
      (Utilities|FlowControl|Sequence
        (:then_0
          (Effects|SpawnEmitteratLocation "/Game/TestTaskContent/Blueprints/CinematicObjects/VFX/P_ky_waterBallHit.P_ky_waterBallHit" (Transformation|GetWorldLocation (Variables|Default|GetStaticMesh)) "0, 0, 0" "6.000000,6.000000,6.000000"))
        (:then_1
          (Components|StaticMesh|SetStaticMesh _staticmesh (Variables|Settings|GetInTransformMesh)))
        (:then_2
          (CallFunction|Move))))
    (:else)))

(fn ConstructionScript)