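; BP_SettingableObjectParent is a parent Blueprint for "settingable" objects that switch between a visible and a hidden ghost state and show an interaction hint.
; ChangeVisibility swaps visibility and query-only collision between StaticMesh and GhostCollision, toggling a "Face" text label with the mesh.
; InteractCollision overlaps by Player-tagged actors add or remove the WBP_InteractHint widget.
; GetVisibility reports the current state from the mesh.
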(event OnComponentBeginOverlap(InteractCollision)
  (params (OverlappedComponent :type Primitive%20Component%20Object%20Reference) (OtherActor :type Actor%20Object%20Reference) (OtherComp :type Primitive%20Component%20Object%20Reference) (OtherBodyIndex :type Integer) (bFromSweep :type Boolean) (SweepResult :type Hit%20Result%20Structure%20%28by%20ref%29))
  (if (Actor|ActorHasTag OtherActor "Player")
    (bind _returnvalue (UserInterface|CreateWidget "/Game/TestTaskContent/UI/WBP_InteractHint.WBP_InteractHint_C"))
    (bind _output_get (Variables|Default|SetInteractHint _returnvalue))
    (UserInterface|Viewport|AddtoViewport _output_get 0)))

(event OnComponentEndOverlap(InteractCollision)
  (params (OverlappedComponent :type Primitive%20Component%20Object%20Reference) (OtherActor :type Actor%20Object%20Reference) (OtherComp :type Primitive%20Component%20Object%20Reference) (OtherBodyIndex :type Integer))
  (if (Actor|ActorHasTag OtherActor "Player")
    (bind _interacthint (Variables|Default|GetInteractHint)
      (:then
        (Widget|RemovefromParent _interacthint)
        (Variables|Default|SetInteractHint 0))
      (:else))))

(event EventBeginPlay)

(event Collision|EventActorBeginOverlap
  (params (OtherActor :type Actor%20Object%20Reference)))

(event EventTick
  (params (DeltaSeconds :type Float%20%28single-precision%29)))

(event EventChangeVisibility
  (params (InVisibility :type Boolean))
  (bind _staticmesh (Variables|Default|GetStaticMesh))
  (bind _ghostcollision (Variables|Default|GetGhostCollision))
  (bind _staticmesh_2 (Variables|Default|GetStaticMesh))
  (bind _ghostcollision_2 (Variables|Default|GetGhostCollision))
  (Variables|Default|GetStaticMesh
    (:then
      (if InVisibility
        ;[1 1 1] Видно
        (Rendering|SetVisibility _staticmesh_2 true false)
        (Collision|SetCollisionEnabled _staticmesh_2 "QueryOnly")
        (Development|SetHiddeninGame _ghostcollision_2 true false)
        (Collision|SetCollisionEnabled _ghostcollision_2 "NoCollision")
        (Rendering|Components|TextRender|SetText (Variables|Default|GetTextRender) (Utilities|Text|MakeLiteralText "Face"))
        (else
          ;[1 1 1] Не видно
          (Rendering|SetVisibility _staticmesh false false)
          (Collision|SetCollisionEnabled _staticmesh "NoCollision")
          (Development|SetHiddeninGame _ghostcollision false false)
          (Collision|SetCollisionEnabled _ghostcollision "QueryOnly")
          (Rendering|Components|TextRender|SetText (Variables|Default|GetTextRender) (Utilities|Text|MakeLiteralText " ")))))
    (:else)))

(fn ConstructionScript)

(fn GetVisibility
  (return (Rendering|IsVisible (Variables|Default|GetStaticMesh))))