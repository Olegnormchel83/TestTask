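; BP_TTPlayerController is the player controller that turns Enhanced Input actions into movement, look, jump, interact and pause for BP_TTCharacter.
; On BeginPlay it caches the possessed character, adds IMC_Default and switches to game-only input with a hidden cursor.
; Movement follows control yaw, while jump and interact are forwarded to the character.
; Pause freezes the game and shows a lazily created, reused WBP_Pause with UI-only input and a visible cursor.
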(event Input|EnhancedActionEvents|EnhancedInputActionIA_Move
  (params (ActionValue :type Vector%202D%20Structure) (ElapsedSeconds :type Float%20%28double-precision%29) (TriggeredSeconds :type Float%20%28double-precision%29) (InputAction :type Input%20Action%20Object%20Reference :default "/Game/TestTaskContent/Core/EnhancedInput/Actions/IA_Move.IA_Move"))
  (bind _ttcharacter (Variables|Default|GetTTCharacter))
  (bind _ttcharacter_2 (Variables|Default|GetTTCharacter)
    (:then
      (Pawn|Input|AddMovementInput _ttcharacter_2 (Math|Vector|GetRightVector (Math|Rotator|MakeRotator (.roll (Pawn|GetControlRotation _ttcharacter_2 :!class /Script/Engine.Pawn)) 0.0 (.yaw (Pawn|GetControlRotation _ttcharacter_2 :!class /Script/Engine.Pawn)))) (.x ActionValue) false)
      (Pawn|Input|AddMovementInput _ttcharacter (Math|Vector|GetForwardVector (Math|Rotator|MakeRotator 0.0 0.0 (.yaw (Pawn|GetControlRotation _ttcharacter :!class /Script/Engine.Pawn)))) (.y ActionValue) false))
    (:else)))

(event Input|EnhancedActionEvents|EnhancedInputActionIA_Look
  (params (ActionValue :type Vector%202D%20Structure) (ElapsedSeconds :type Float%20%28double-precision%29) (TriggeredSeconds :type Float%20%28double-precision%29) (InputAction :type Input%20Action%20Object%20Reference :default "/Game/TestTaskContent/Core/EnhancedInput/Actions/IA_Look.IA_Look"))
  (Class|PlayerController|AddYawInput (.x ActionValue))
  (Class|PlayerController|AddPitchInput (.y ActionValue)))

(event Input|EnhancedActionEvents|EnhancedInputActionIA_Jump
  (params (ActionValue :type Boolean) (ElapsedSeconds :type Float%20%28double-precision%29) (TriggeredSeconds :type Float%20%28double-precision%29) (InputAction :type Input%20Action%20Object%20Reference :default "/Game/TestTaskContent/Core/EnhancedInput/Actions/IA_Jump.IA_Jump"))
  (:Started
    (bind _ttcharacter (Variables|Default|GetTTCharacter)
      (:then
        (Character|Jump _ttcharacter))
      (:else)))
  (:Completed
    (bind _ttcharacter_2 (Variables|Default|GetTTCharacter)
      (:then
        (Character|StopJumping _ttcharacter_2))
      (:else))))

(event Input|EnhancedActionEvents|EnhancedInputActionIA_Pause
  (params (ActionValue :type Boolean) (ElapsedSeconds :type Float%20%28double-precision%29) (TriggeredSeconds :type Float%20%28double-precision%29) (InputAction :type Input%20Action%20Object%20Reference :default "/Game/TestTaskContent/Core/EnhancedInput/Actions/IA_Pause.IA_Pause"))
  (if (not (Game|IsGamePaused))
    (Game|SetGamePaused true)
    (Utilities|IsValid (Variables|Default|GetPauseWidget)
      (:Is%20Valid
        _)
      (:Is%20Not%20Valid
        (bind _returnvalue (UserInterface|CreateWidget "/Game/TestTaskContent/UI/WBP_Pause.WBP_Pause_C"))
        (Variables|Default|SetPauseWidget _returnvalue)))
    (UserInterface|Viewport|AddtoViewport (Variables|Default|GetPauseWidget) 0)
    (Input|SetInputModeUIOnly self 0 "DoNotLock" false)
    (Variables|Default|SetbShowMouseCursor true)))

(event Input|EnhancedActionEvents|EnhancedInputActionIA_Interact
  (params (ActionValue :type Boolean) (ElapsedSeconds :type Float%20%28double-precision%29) (TriggeredSeconds :type Float%20%28double-precision%29) (InputAction :type Input%20Action%20Object%20Reference :default "/Game/TestTaskContent/Core/EnhancedInput/Actions/IA_Interact.IA_Interact"))
  (:Started
    (bind _ttcharacter (Variables|Default|GetTTCharacter)
      (:then
        (Default|TrytoInteract _ttcharacter))
      (:else))))

(event EventBeginPlay
  (Utilities|FlowControl|Sequence
    (:then_0
      (bind _asbp_ttcharacter (Utilities|Casting|CastToBP_TTCharacter (Pawn|GetControlledPawn)))
      (bind _output_get (Variables|Default|SetTTCharacter _asbp_ttcharacter))
      (Variables|Default|SetCharacter%20Movement (Variables|/Script/Engine.Character|GetCharacterMovement _output_get)))
    (:then_1
      (Input|AddMappingContext (PlayerController|LocalPlayerSubsystems|GetEnhancedInputLocalPlayerSubsystem) "/Game/TestTaskContent/Core/EnhancedInput/IMC_Default.IMC_Default" 0 "(bIgnoreAllPressedKeysUntilRelease=True,bForceImmediately=False,bNotifyUserSettings=False)"))
    (:then_2
      (Input|SetInputModeGameOnly self false)
      (Variables|Default|SetbShowMouseCursor false))))

(fn ConstructionScript)